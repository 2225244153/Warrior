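; Player character Blueprint that grants a base Gameplay Ability on BeginPlay and handles third-person mouse look.
; Yaw input passes straight through, while pitch input applies only if the predicted control pitch stays within a limited range, handling the 360-degree wrap.
; LockCamera toggles between free spring-arm orbit with movement-oriented rotation and an offset camera with the character following controller yaw.
; Movement, jump and montage nodes are present but unconnected.
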(event Collision|EventActorBeginOverlap
  (params (OtherActor :type Actor%20Object%20Reference)))

(event EventTick
  (params (DeltaSeconds :type Float%20%28single-precision%29)))

(event EventBeginPlay
  (GameplayAbilities|GiveAbility (Variables|Default|GetAbilitySystemComponent) "/Game/A_Game/Abilities/GAB_BaseAbility.GAB_BaseAbility_C" 0 -1))

(event Input|ActionEvents|InputActionJump
  (params (Key :type Key%20Structure :default "None"))
  ;[1 1 1] 跳跃
)

(event Input|AxisEvents|InputAxisTurnRight/LeftMouse
  (params (AxisValue :type Float%20%28single-precision%29))
  ;[1 1 1] 鼠标的上下左右看
  (Pawn|Input|AddControllerYawInput AxisValue))

(event Input|AxisEvents|InputAxisLookUp/DownMouse
  (params (AxisValue :type Float%20%28single-precision%29))
  (bind _returnvalue (Game|GetPlayerController 0))
  (bind _returnvalue_2 (Pawn|GetControlRotation _returnvalue :!class /Script/Engine.Controller))
  (bind _returnvalue_3 (Class|PlayerController|GetDeprecatedInputPitchScale _returnvalue))
  (bind _returnvalue_4 (* AxisValue _returnvalue_3))
  (bind _returnvalue_5 (+ _returnvalue_4 (.pitch _returnvalue_2)))
  (if (or (< _returnvalue_5 4e+01) (and (<= _returnvalue_5 3.6e+02) (>= _returnvalue_5 3e+02)))
    ;[1 1 1] 鼠标的上下左右看
    (Pawn|Input|AddControllerPitchInput AxisValue)))

(fn ConstructionScript)

(fn LockCamera
  (params (Lock :type Boolean))
  (bind _springarm (Variables|Default|GetSpringArm))
  (bind _charactermovement (Variables|Character|GetCharacterMovement))
  (bind _camera (Variables|Default|GetCamera))
  (if Lock
    (Variables|/Script/Engine.SpringArmComponent|SetbUsePawnControlRotation _springarm false)
    (Variables|/Script/Engine.CharacterMovementComponent|SetbOrientRotationToMovement _charactermovement false)
    (Variables|Default|SetbUseControllerRotationYaw true)
    (Transformation|SetRelativeTransform _camera (Math|Transform|MakeTransform "0.000000,0.000000,200.000000" "-20.000000,0.000000,0.000000" "1.000000,1.000000,1.000000") false false)
    (else
      (Variables|/Script/Engine.SpringArmComponent|SetbUsePawnControlRotation _springarm true)
      (Variables|/Script/Engine.CharacterMovementComponent|SetbOrientRotationToMovement _charactermovement true)
      (Variables|Default|SetbUseControllerRotationYaw false)
      (Transformation|SetRelativeTransform _camera (Math|Transform|MakeTransform "0, 0, 0" "0, 0, 0" "1.000000,1.000000,1.000000") false false))))